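; BP_HoverSeagull is a player-driven seagull that hovers and is pushed forward with physics forces.
; Four hover components at the beak, tail and both wings are each initialized with the seagull mesh on BeginPlay.
; The MoveForward input axis adds a large force along the mesh's forward vector, with no turning input in this graph.
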(event `self.ReceiveBeginPlay`
  (bind _hoverseagullmesh (`self.HoverSeagullMesh`))
  (`/Game/Blueprints/Hovering/HoverComponent.InitComponent` (`self.HoverComponentBeak`) _hoverseagullmesh)
  (`/Game/Blueprints/Hovering/HoverComponent.InitComponent` (`self.HoverComponentTail`) _hoverseagullmesh)
  (`/Game/Blueprints/Hovering/HoverComponent.InitComponent` (`self.HoverComponentLeftWing`) _hoverseagullmesh)
  (`/Game/Blueprints/Hovering/HoverComponent.InitComponent` (`self.HoverComponentRightWing`) _hoverseagullmesh))

(event `InputAxis|MoveForward`
  (params (AxisValue :type "Float (single-precision)"))
  (`PrimitiveComponent.AddForce` (`self.HoverSeagullMesh`) (* (* (`SceneComponent.GetForwardVector` (`self.HoverSeagullMesh`)) 500000.0) AxisValue) "None" false))

(fn `UserConstructionScript`)